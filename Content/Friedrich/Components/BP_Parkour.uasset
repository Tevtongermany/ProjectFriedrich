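; Parkour component that gives a Character wall running, sprinting, crouching and sliding, with jump handling for each.
; Looping timers tilt the camera and drive gated updates, toggled by jump, landing and movement-mode events.
; A parkour mode tracks state, restores cached movement defaults and lets queued slides or sprints resume on landing.
; Wall runs use side traces and launches along the wall; slides use a plane constraint and slope-based impulse.
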(event `On Update`
  ;[1 1 1] Update
  (`|ExecutionSequence`
    (:`then_0`
      (`/Engine/EditorBlueprintResources/StandardMacros.Gate` true :!label _label
        (:`Exit`
          (`self.WallRunUpdate`))))
    (:`then_1`
      (`/Engine/EditorBlueprintResources/StandardMacros.Gate` true :!label _label_2
        (:`Exit`
          (`self.Sprint Update`))))
    (:`then_2`
      (`/Engine/EditorBlueprintResources/StandardMacros.Gate` true :!label _label_3
        (:`Exit`
          (`self.Slide Update`))))))

(event `OpenWallRunGate`
  ;[1 1 1] Update
  (goto _label :!via `Open`))

(event `CloseWallRunGate`
  ;[1 1 1] Update
  (goto _label :!via `Close`))

(event `Open Sprint Gate`
  ;[1 1 1] Update
  (set `self.Is Sprint Gate open?` true)
  (goto _label_2 :!via `Open`))

(event `Close Sprint Gate`
  ;[1 1 1] Update
  (goto _label_2 :!via `Close`))

(event `Init`
  (params (Character :type "Character Object Reference"))
  (bind _character_movement (`self.Character Movement`))
  ;[1 1 1] Update
  (bind _output_get (set `self.Character` Character))
  (bind _output_get_2 (set `self.Character Movement` (`Character.CharacterMovement` _output_get)))
  (set `self.Default Gravity` (`CharacterMovementComponent.GravityScale` _output_get_2))
  (set `self.Character Capsule Component` (`Character.CapsuleComponent` (`self.Character`)))
  (set `self.Default Ground Friction` (`CharacterMovementComponent.GroundFriction` _character_movement))
  (set `self.Default Braking Deceleration` (`CharacterMovementComponent.BrakingDecelerationWalking` _character_movement))
  (set `self.Default Crouch Speed` (`CharacterMovementComponent.MaxWalkSpeedCrouched` _character_movement))
  (set `self.Default Max Walk Speed` (`CharacterMovementComponent.MaxWalkSpeed` (`self.Character Movement`)))
  (`KismetSystemLibrary.K2_SetTimerDelegate` (delegate `On Update`) 0.01 true))

(event `SlideGateOpen`
  ;[1 1 1] Update
  (set `self.Is Slide Gate open?` true)
  (goto _label_3 :!via `Open`))

(event `SlideGate Closed`
  ;[1 1 1] Update
  (set `self.Is Slide Gate open?` true)
  (goto _label_3 :!via `Close`))

(event `ResetWallRunSuppression`
  ;[1 1 1] Idk if this is used anymore lol
  (`KismetSystemLibrary.K2_ClearTimer` null "ResetWallRunSuppression") ; if This shit changes change the name in SupresswallRun Function aswell!!
  (set `self.WallRunSuppressed?` false)
  (`self.On Wall Run End`))

(event `self.ReceiveBeginPlay`
  ;[1 1 1] Idfk what this means
  (`KismetSystemLibrary.K2_SetTimerDelegate` (delegate `Camera Tick Event`) 0.01 true))

(event `On Land Event`
  ;[1 1 1] On Land events
  (`self.End Events`)
  (`self.Close Gates`))

(event `Camera Tick Event`
  (bind _current_parkour_mode (`self.Current Parkour Mode`))
  ;[1 1 1] Idfk what this means
  (if (`|EnumEquality` _current_parkour_mode "NewEnumerator1")
    (`self.Camera Tilt` 15.0)
    (elif (`|EnumEquality` _current_parkour_mode "NewEnumerator3")
      (`self.Camera Tilt` -15.0)
      (else
        (`self.Camera Tilt` 0.0)))))

(event `On Jump Event`
  ;[1 1 1] On Jump event
  (if (`|EnumEquality` (`self.Current Parkour Mode`) "NewEnumerator0")
    (if (not (`NavMovementComponent.IsFalling` (`self.Character Movement`)))
      (`self.Open Gates`)
      (`KismetSystemLibrary.PrintString` "Open Gates Event"))
    (else
      (`self.Jump Events`)
      (`KismetSystemLibrary.PrintString` "Jump event"))))

(event `Crouch Slide Event`
  ;[1 1 1] Crouch Slide Stuff
  (if (`self.Is Wall Running?`)
    (`self.Wall Run End` 0.5)
    (elif (`NavMovementComponent.IsFalling` (`self.Character Movement`))
      (set `self.SlideQueued` true)
      (elif (`self.Can Slide`)
        (if (`CharacterMovementComponent.IsWalking` (`self.Character Movement`))
          (`self.Slide Start`)
          (else
            (set `self.SlideQueued` false)))
        (else
          (switch `/Game/Friedrich/Enum/EParkourMode` (`self.Current Parkour Mode`)
            (:`NewEnumerator0`
              (`self.Crouch Start`))
            (:`NewEnumerator5`
              (`self.Crouch End`))))))))

(event `CheckQueues`
  ;[1 1 1] Queses
  (if (`self.SlideQueued`)
    (`self.Slide Start`)
    (elif (`self.SprintQueued`)
      (`self.Sprint Start`))))

(event `ParkourMovementChanged`
  (params (PrevParkourMode :type "/Game/Friedrich/Enum/EParkourMode Enum" :default "NewEnumerator0") (NewParkourMode :type "/Game/Friedrich/Enum/EParkourMode Enum" :default "NewEnumerator0"))
  ;[1 1 1] Change Events
  (set `self.Previous Parkour Mode` PrevParkourMode)
  (set `self.Current Parkour Mode` NewParkourMode)
  (`self.Reset Movement`))

(event `Sprint Event`
  ;[1 1 1] Sprint
  (`self.Sprint Start`))

(event `MovementChanged`
  (params (PrevMovementMode :type "EMovementMode Enum" :default "MOVE_None") (NewMovementMode :type "EMovementMode Enum" :default "MOVE_None"))
  ;[1 1 1] Change Events
  (`/Engine/EditorBlueprintResources/StandardMacros.IsValid` (`self.Character Movement`)
    (:`Is Valid`
      (set `self.PrevMovementMode` PrevMovementMode)
      (set `self.CurrentMovementMode` NewMovementMode)
      (if (and (`|EnumEquality` (`self.PrevMovementMode`) "MOVE_Walking") (`|EnumEquality` (`self.CurrentMovementMode`) "MOVE_Falling"))
        (`self.Sprint Jump`)
        (`self.End Events`)
        (`self.Open Gates`)
        (elif (and (`|EnumEquality` (`self.PrevMovementMode`) "MOVE_Falling") (`|EnumEquality` (`self.CurrentMovementMode`) "MOVE_Walking"))
          (`self.CheckQueues`))))))

(fn `Camera Tilt`
  (params (`Target X (Roll)` :type "Float (double-precision)"))
  (bind _returnvalue (`Controller.GetControlRotation` (`Pawn.GetController` (`self.Character`))))
  (`Controller.SetControlRotation` (`Pawn.GetController` (`self.Character`)) (`KismetMathLibrary.RInterpTo` _returnvalue (`KismetMathLibrary.MakeRotator` `Target X (Roll)` (.pitch _returnvalue) (.yaw _returnvalue)) (`GameplayStatics.GetWorldDeltaSeconds`) 10.0)))

(fn `Close Gates`
  (`self.Close Sprint Gate`)
  (`self.SlideGate Closed`)
  (`self.CloseWallRunGate`))

(fn `Crouch End`
  (if (`|EnumEquality` (`self.Current Parkour Mode`) "NewEnumerator5")
    (`Character.UnCrouch` (`self.Character`))
    (`self.Set Parkour Movement Mode` "NewEnumerator0")
    (set `self.SprintQueued` false)
    (set `self.SlideQueued` false)))

(fn `Crouch Jump`
  (if (`|EnumEquality` (`self.Current Parkour Mode`) "NewEnumerator5")
    (`self.Crouch End`)))

(fn `Crouch Start`
  (if (`self.Parkour Mode None?`)
    (`Character.Crouch` (`self.Character`))
    (`self.Set Parkour Movement Mode` "NewEnumerator5")
    (set `self.SprintQueued` false)
    (set `self.SlideQueued` false)))

(fn `End Events`
  (`self.Sprint End`)
  (`self.Wall Run End` 0.1)
  (`self.Slide End` false)
  (`self.Crouch End`))

(fn `Jump Events`
  (`self.WallRunJump`)
  (`self.Slide Jump`)
  (`self.Crouch Jump`)
  (`self.Sprint Jump`))

(fn `Open Gates`
  (`KismetSystemLibrary.PrintString` "Should Open Wall run Gate")
  (`self.OpenWallRunGate`)
  (`self.Open Sprint Gate`)
  (`self.SlideGateOpen`))

(fn `Reset Movement`
  (bind _current_parkour_mode (`self.Current Parkour Mode`))
  (bind _character_movement (`self.Character Movement`))
  (if (or (`|EnumEquality` _current_parkour_mode "NewEnumerator0") (`|EnumEquality` _current_parkour_mode "NewEnumerator5"))
    (set `CharacterMovementComponent.GravityScale` (`self.Default Gravity`) (`self.Character Movement`))
    (set `CharacterMovementComponent.GroundFriction` (`self.Default Ground Friction`) (`self.Character Movement`))
    (set `CharacterMovementComponent.BrakingDecelerationWalking` (`self.Default Braking Deceleration`) _character_movement)
    (set `CharacterMovementComponent.MaxWalkSpeed` (`self.Default Max Walk Speed`) _character_movement)
    (set `CharacterMovementComponent.MaxWalkSpeedCrouched` (`self.Default Crouch Speed`) _character_movement)
    (`MovementComponent.SetPlaneConstraintEnabled` (`self.Character Movement`) false)
    (`CharacterMovementComponent.SetMovementMode` (`self.Character Movement`) (select `/Game/Friedrich/Enum/EParkourMode` (`self.Previous Parkour Mode`) :`NewEnumerator0` "MOVE_Walking" :`NewEnumerator1` "MOVE_Falling" :`NewEnumerator3` "MOVE_Falling" :`NewEnumerator4` "MOVE_Falling" :`NewEnumerator5` "MOVE_Walking" :`NewEnumerator6` "MOVE_Walking" :!type "EMovementMode Enum") 0)))

(fn `Set Parkour Movement Mode`
  (params (`New Mode` :type "/Game/Friedrich/Enum/EParkourMode Enum" :default "NewEnumerator0"))
  (returns (Changed :type Boolean))
  (if (`|EnumEquality` (`self.Current Parkour Mode`) `New Mode`)
    (return false)
    (else
      (`self.ParkourMovementChanged` (`self.Current Parkour Mode`) `New Mode`)
      (return true))))

(fn `Slide End`
  (params (Crouch :type Boolean))
  (if (`|EnumEquality` (`self.Current Parkour Mode`) "NewEnumerator4")
    (bind _changed (`self.Set Parkour Movement Mode` (select `bool` Crouch :`false` "NewEnumerator0" :`true` "NewEnumerator5" :!type "/Game/Friedrich/Enum/EParkourMode Enum")))
    (if _changed
      (`self.SlideGate Closed`)
      (if (not (`local.Crouch`))
        (`Character.UnCrouch` (`self.Character`))))))

(fn `Slide Jump`
  (if (`|EnumEquality` (`self.Current Parkour Mode`) "NewEnumerator4")
    (`self.Slide End` false)
    (if (`NavMovementComponent.IsFalling` (`self.Character Movement`))
      (`Character.LaunchCharacter` (`self.Character`) (`KismetMathLibrary.MakeVector` 0.0 0.0 (`CharacterMovementComponent.JumpZVelocity` (`self.Character Movement`))) false false)
      (set `self.SlideQueued` true))))

(fn `Slide Start`
  (bind _character_movement (`self.Character Movement`))
  (if (and (`self.Can Slide`) (`CharacterMovementComponent.IsWalking` (`self.Character Movement`)))
    (`self.Sprint End`)
    (`self.Set Parkour Movement Mode` "NewEnumerator4")
    (`Character.Crouch` (`self.Character`))
    (set `CharacterMovementComponent.GroundFriction` 0.0 _character_movement)
    (set `CharacterMovementComponent.BrakingDecelerationWalking` 1400.0 _character_movement)
    (set `CharacterMovementComponent.MaxWalkSpeedCrouched` 0.0 _character_movement)
    (`MovementComponent.SetPlaneConstraintFromVectors` _character_movement (`KismetMathLibrary.Normal` (`MovementComponent.Velocity` _character_movement)) (`Actor.GetActorUpVector` (`self.Character`)))
    (`MovementComponent.SetPlaneConstraintEnabled` _character_movement true)
    (bind _returnvalue (`self.Get Wall Run Vector`))
    (if (<= (.z _returnvalue) 0.02)
      (`CharacterMovementComponent.AddImpulse` (`self.Character Movement`) (* _returnvalue (`self.Slide Impulse Amount`)) true))
    (`self.SlideGateOpen`)
    (set `self.SprintQueued` false)
    (set `self.SlideQueued` false)))

(fn `Slide Update`
  (if (`|EnumEquality` (`self.Current Parkour Mode`) "NewEnumerator4")
    (if (<= (`KismetMathLibrary.VSize` (`MovementComponent.Velocity` (`self.Character Movement`))) 0.36)
      (`self.Slide End` true))))

(fn `Sprint End`
  (`KismetSystemLibrary.PrintString` "Sprint End Event")
  (if (`|EnumEquality` (`self.Current Parkour Mode`) "NewEnumerator6")
    (bind _changed (`self.Set Parkour Movement Mode` "NewEnumerator0"))
    (if _changed
      (`self.Close Sprint Gate`)
      (`KismetSystemLibrary.K2_SetTimer` null "Open Sprint Gate" 0.1)
      (`KismetSystemLibrary.PrintString` "yes")
      (else
        (`KismetSystemLibrary.PrintString` "hurensohn bad code >:(")))))

(fn `Sprint Jump`
  (if (`|EnumEquality` (`self.Current Parkour Mode`) "NewEnumerator6")
    (`self.Sprint End`)
    (set `self.SprintQueued` true)
    (`KismetSystemLibrary.PrintString` "Sprint Jump Event")))

(fn `Sprint Start`
  (`self.Slide End` false)
  (`self.Crouch End`)
  (if (`self.Can Sprint`)
    (bind _changed (`self.Set Parkour Movement Mode` "NewEnumerator6"))
    (if _changed
      (set `CharacterMovementComponent.MaxWalkSpeed` (`self.Sprint Speed`) (`self.Character Movement`))
      (`self.Open Sprint Gate`)
      (set `self.SprintQueued` false)
      (set `self.SlideQueued` false))))

(fn `Sprint Update`
  (if (`|EnumEquality` (`self.Current Parkour Mode`) "NewEnumerator6")
    (if (not (> (`self.ForwardInput`) 0.0))
      (`self.Sprint End`))))

(fn `SupressWallRun`
  (params (delay :type "Float (double-precision)"))
  (set `self.WallRunSuppressed?` true)
  (`KismetSystemLibrary.K2_SetTimer` null "ResetWallRunSuppression" delay))

(fn `Wall Run End`
  (params (`Reset Time` :type "Float (double-precision)"))
  (if (`self.Is Wall Running?`)
    (bind _changed (`self.Set Parkour Movement Mode` "NewEnumerator0"))
    (if _changed
      (`self.CloseWallRunGate`)
      (`KismetSystemLibrary.K2_SetTimer` null "OpenWallRunGate" `Reset Time`))))

(fn `Wall Run Gravity`
  (bind _character_movement (`self.Character Movement`))
  (set `CharacterMovementComponent.GravityScale` (`KismetMathLibrary.FInterpTo` (`CharacterMovementComponent.GravityScale` _character_movement) (`self.WallRun Target Gravity`) (`GameplayStatics.GetWorldDeltaSeconds`) 10.0) _character_movement))

(fn `WallRunJump`
  (if (`self.Is Wall Running?`)
    (`self.Wall Run End` 0.3)
    (`Character.LaunchCharacter` (`self.Character`) (`KismetMathLibrary.MakeVector` (* (`self.WallRunJumpOffForce`) (.x (`self.WallRunNormal`))) (* (`self.WallRunJumpOffForce`) (.y (`self.WallRunNormal`))) (`self.WallRunJumpHeight`)) false true)
    (`GameplayStatics.PlaySoundAtLocation` (`self.Wall Run Jump Off Sound`) (`Actor.K2_GetActorLocation` (`self.Character`)) (struct) 1.0 1.0 0.0 null null null)))

(fn `WallRunMovement`
  (params (Start :type "Vector Structure") (End :type "Vector Structure") (Direction :type "Float (double-precision)"))
  (returns (`On wall` :type Boolean))
  (bind _character (`self.Character`))
  (bind _outhit (`KismetSystemLibrary.LineTraceSingle` Start End "TraceTypeQuery1"))
  (bind (_bblockinghit _binitialoverlap _time _distance _location _impactpoint _normal) (`GameplayStatics.BreakHitResult` _outhit))
  (if _bblockinghit
    (if (`Actor.ActorHasTag` (`.HitActor` (`GameplayStatics.BreakHitResult` _outhit)) "NoWallRunPossible")
      (return false)
      (else
        (bind (_returnvalue _out_vector) (`self.ValidWallRunVector` _normal))
        (if (and (`NavMovementComponent.IsFalling` (`self.Character Movement`)) _returnvalue)
          (set `self.WallRunNormal` _out_vector)
          (`Character.LaunchCharacter` _character (`self.PlayerToWallVector`) false false)
          (`Character.LaunchCharacter` _character (* (`KismetMathLibrary.Cross_VectorVector` (`self.WallRunNormal`) (0.0 0.0 1.0)) (* (select `bool` (`self.SprintQueued`) :`false` (`self.Wall Run Speed`) :`true` (`self.Wall Run Sprint Speed`)) (`local.Direction`))) true (not (`self.Should Have Gravity?`)))
          (return true)
          (else
            (return false)))))
    (else
      (return false))))

(fn `WallRunUpdate`
  (if (`self.Can Wall Run`)
    (bind _on_wall (`self.WallRunMovement` (`Actor.K2_GetActorLocation` (`self.Character`)) (`self.WallRunEndVectors`) -1.0))
    (if _on_wall
      (`self.Set Parkour Movement Mode` "NewEnumerator3")
      (`self.Wall Run Gravity` :!label _label)
      (`self.On Wall Run Start`)
      (elif (`|EnumEquality` (`self.Current Parkour Mode`) "NewEnumerator3")
        (`self.Wall Run End` 1.0)
        (else
          (bind _on_wall_2 (`self.WallRunMovement` (`Actor.K2_GetActorLocation` (`self.Character`)) (`.Left` (`self.WallRunEndVectors`)) 1.0))
          (if _on_wall_2
            (`self.Set Parkour Movement Mode` "NewEnumerator1")
            (goto _label)
            (else
              (`GameplayStatics.PlaySoundAtLocation` (`self.Wall Run Jump Off Sound`) (`Actor.K2_GetActorLocation` (`self.Character`)) (struct) 1.0 1.0 0.0 null null null)
              (`self.Wall Run End` 1.0))))))
    (else
      (`self.Wall Run End` 1.0))))