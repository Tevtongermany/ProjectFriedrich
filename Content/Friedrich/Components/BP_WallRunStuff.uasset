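; Character component that adds wall running, wall jumping and camera tilt.
; After Init, a looping timer traces right and left for near-vertical walls while the character falls, launching it along the wall and easing gravity toward a target.
; Ending a run restores gravity and briefly suppresses re-attachment; jumping launches off the wall normal.
; A separate timer interpolates control-rotation roll according to the wall side.
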(event `ResetWallRunSuppression`
  (`KismetSystemLibrary.K2_ClearTimer` null "ResetWallRunSuppression") ; if This shit changes change the name in SupresswallRun Function aswell!!
  (set `self.WallRunSuppressed?` false)
  (`self.On Wall Run End`))

(event `On Land Event`
  (`self.Wall Run End` 0.0)
  (set `self.WallRunSuppressed?` false))

(event `On Jump Event`
  (`self.WallRunJump`))

(event `OnWallRunUpdate`
  (if (not (`self.WallRunSuppressed?`))
    (`self.WallRunUpdate`)))

(event `Init`
  (params (Character :type "Character Object Reference"))
  (bind _output_get (set `self.Character` Character))
  (bind _output_get_2 (set `self.Character Movement` (`Character.CharacterMovement` _output_get)))
  (set `self.Default Gravity` (`CharacterMovementComponent.GravityScale` _output_get_2))
  (`KismetSystemLibrary.K2_SetTimerDelegate` (delegate `OnWallRunUpdate`) 0.02 true))

(event `self.ReceiveBeginPlay`
  (`KismetSystemLibrary.K2_SetTimerDelegate` (delegate `Camera Tick Event`) 0.01 true))

(event `Camera Tick Event`
  (if (`self.WallRunningOnLeft`)
    (`self.Camera Tilt` 15.0)
    (elif (`self.WallRunningOnRight`)
      (`self.Camera Tilt` -15.0)
      (else
        (`self.Camera Tilt` 0.0)))))

(fn `Camera Tilt`
  (params (`Target X (Roll)` :type "Float (double-precision)"))
  (bind _returnvalue (`Controller.GetControlRotation` (`Pawn.GetController` (`self.Character`))))
  (`Controller.SetControlRotation` (`Pawn.GetController` (`self.Character`)) (`KismetMathLibrary.RInterpTo` _returnvalue (`KismetMathLibrary.MakeRotator` `Target X (Roll)` (.pitch _returnvalue) (.yaw _returnvalue)) (`GameplayStatics.GetWorldDeltaSeconds`) 10.0)))

(fn `SupressWallRun`
  (params (delay :type "Float (double-precision)"))
  (set `self.WallRunSuppressed?` true)
  (`KismetSystemLibrary.K2_SetTimer` null "ResetWallRunSuppression" delay))

(fn `Wall Run End`
  (params (`Reset Time` :type "Float (double-precision)"))
  (if (`self.isWallRunning?`)
    (set `self.isWallRunning?` false)
    (set `self.WallRunningOnRight` false)
    (set `self.WallRunningOnLeft` false)
    (set `CharacterMovementComponent.GravityScale` (`self.Default Gravity`) (`self.Character Movement`))
    (`self.SupressWallRun` `Reset Time`)))

(fn `WallRunJump`
  (if (`self.isWallRunning?`)
    (`self.Wall Run End` 0.3)
    (`Character.LaunchCharacter` (`self.Character`) (`KismetMathLibrary.MakeVector` (* (`self.WallRunJumpOffForce`) (.x (`self.WallRunNormal`))) (* (`self.WallRunJumpOffForce`) (.y (`self.WallRunNormal`))) (`self.WallRunJumpHeight`)) false true)))

(fn `WallRunMovement`
  (params (Start :type "Vector Structure") (End :type "Vector Structure") (Direction :type "Float (double-precision)"))
  (returns (`On wall` :type Boolean))
  (bind _character (`self.Character`))
  (bind _outhit (`KismetSystemLibrary.LineTraceSingle` Start End "TraceTypeQuery1"))
  (bind (_bblockinghit _binitialoverlap _time _distance _location _impactpoint _normal) (`GameplayStatics.BreakHitResult` _outhit))
  (if _bblockinghit
    (bind (_returnvalue _out_vector) (`self.ValidWallRunVector` _normal))
    (if (and (`NavMovementComponent.IsFalling` (`self.Character Movement`)) _returnvalue)
      (set `self.WallRunNormal` _out_vector)
      (`Character.LaunchCharacter` _character (`self.PlayerToWallVector`) false false)
      (`Character.LaunchCharacter` _character (* (`KismetMathLibrary.Cross_VectorVector` (`self.WallRunNormal`) (0.0 0.0 1.0)) (* (`self.Wall Run Speed`) (`local.Direction`))) true (not (`self.Should Have Gravity?`)))
      (return true)
      (else
        (return false)))
    (else
      (return false))))

(fn `WallRunUpdate`
  (bind _on_wall (`self.WallRunMovement` (`Actor.K2_GetActorLocation` (`self.Character`)) (`self.WallRunEndVectors`) -1.0))
  (if _on_wall
    (bind _output_get (set `self.isWallRunning?` true))
    (set `self.WallRunningOnRight` _output_get)
    (set `self.WallRunningOnLeft` false)
    (set `CharacterMovementComponent.GravityScale` (`KismetMathLibrary.FInterpTo` (`CharacterMovementComponent.GravityScale` (`self.Character Movement`)) (`self.WallRun Target Gravity`) (`GameplayStatics.GetWorldDeltaSeconds`) 10.0) (`self.Character Movement`) :!label _label)
    (elif (`self.WallRunningOnRight`)
      (`self.Wall Run End` 1.0)
      (else
        (bind _on_wall_2 (`self.WallRunMovement` (`Actor.K2_GetActorLocation` (`self.Character`)) (`.Left` (`self.WallRunEndVectors`)) 1.0))
        (if _on_wall_2
          (set `self.isWallRunning?` true)
          (set `self.WallRunningOnRight` false)
          (set `self.WallRunningOnLeft` true)
          (goto _label)
          (else
            (`self.Wall Run End` 1.0)))))))