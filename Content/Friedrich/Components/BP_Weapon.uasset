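; BP_Weapon is a weapon component that manages which weapon slot a character has equipped.
; Init stores the character and its weapon-holding Child Actor Component, then equips the first slot.
; SwitchToWeapon swaps the child actor class to the slot's weapon Blueprint, then copies that slot's clip and total ammo onto the spawned BP_Parent_Weapon.
; The SwitchWeapon event, BeginPlay and Tick are empty.
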(event `Init`
  (params (`Weapon Holding Actor` :type "ChildActorComponent Object Reference") (Character :type "Character Object Reference"))
  (set `self.Weapon Holding Actor` `Weapon Holding Actor`)
  (set `self.Character` Character)
  (`self.Switch to Weapon` 0))

(event `Switch Weapon`
  (params (`Weapon Index` :type Integer)))

(fn `Switch to Weapon`
  (params (`Weapon Index` :type Integer))
  (bind _output (`|GetArrayItem` (`self.Weapon Slots`) `Weapon Index`))
  (bind (_weapon _totalammo _ammoinsideclip) (break `/Game/Friedrich/Struct/BPS_WeaponSlot` _output))
  (set `self.Current Weapon Slots` _output)
  (`ChildActorComponent.SetChildActorClass` (`self.Weapon Holding Actor`) (`/Game/Friedrich/DataAssets/FriedrichWeaponDefenition.Weapon Blueprint` _weapon))
  (bind _asbp_parent_weapon (cast `/Game/Friedrich/Blueprints/Weapons/BP_Parent_Weapon` (`ChildActorComponent.ChildActor` (`self.Weapon Holding Actor`))))
  (set `/Game/Friedrich/Blueprints/Weapons/BP_Parent_Weapon.Ammo In Clip` _ammoinsideclip _asbp_parent_weapon)
  (set `/Game/Friedrich/Blueprints/Weapons/BP_Parent_Weapon.Total Ammo` _totalammo _asbp_parent_weapon)
  (set `self.currentWeaponSlotIndex` `Weapon Index`))